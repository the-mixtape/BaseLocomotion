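; Blueprint that copies a referenced directional light's forward vector into the MPC_DirectionLight material parameter collection, in the cel shading folder.
; The construction script runs the update, which writes the "Direction Light" vector parameter only when the light reference is valid.
; The DynamicDirectionLight flag works opposite to its name: when true it updates on BeginPlay, and when false it updates every Tick.
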(event Custom|UpdateDirectionLight
  (bind _directionlight (Variables|Default|GetDirectionLight))
  (bind _lightcomponent (Variables|/Script/Engine.Light|GetLightComponent _directionlight))
  (bind _returnvalue (Math|Vector|GetForwardVector _lightcomponent))
  (Utilities|IsValid (Variables|Default|GetDirectionLight)
    (:Is%20Valid
      (Rendering|Material|SetVectorParameterValue "/Game/BaseLocomotion/Materials/Collections/MPC_DirectionLight.MPC_DirectionLight" "Direction Light" (Utilities|Struct|MakeLinearColor (.x _returnvalue) (.y _returnvalue) (.z _returnvalue) 1.0) :!class /Script/Engine.KismetMaterialLibrary))))

(event EventBeginPlay
  (if (Variables|Default|GetDynamicDirectionLight)
    (CallFunction|UpdateDirectionLight)))

(event EventTick
  (params (DeltaSeconds :type Float%20%28single-precision%29))
  (if (not (Variables|Default|GetDynamicDirectionLight))
    (CallFunction|UpdateDirectionLight)))

(fn ConstructionScript
  (CallFunction|UpdateDirectionLight))